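; Tree scatter actor that fills a circle around itself with instances of a chosen mesh.
; The construction script adds TreeAmount-driven instances at unseeded random flat offsets, all with the same stretched scale and no rotation.
; Offsets come from a square and are clamped to Radius, so corner points collect on the rim.
; It then briefly draws a red debug circle showing the radius.
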(event `self.ReceiveTick`
  (params (DeltaSeconds :type "Float (single-precision)")))

(event `DisplayCircle`
  (`KismetSystemLibrary.DrawDebugCircle` (`self.K2_GetActorLocation`) (`self.Radius`) 36 (struct :`R` 1.0 :`A` 1.0) 0.5 0.0 (1.0 0.0 0.0) (0.0 1.0 0.0) true))

(fn `UserConstructionScript`
  (bind _radius (`self.Radius`))
  (bind _returnvalue (* (`self.Radius`) -1.0))
  (`|ExecutionSequence`
    (:`then_0`
      (`StaticMeshComponent.SetStaticMesh` (`self.InstancedStaticMesh`) (`self.ScatterMesh`))
      (for _ (range (+ (`self.TreeAmount`) 1))
        (`InstancedStaticMeshComponent.AddInstance` (`self.InstancedStaticMesh`) (`KismetMathLibrary.MakeTransform` (`KismetMathLibrary.ClampVectorSize` (`KismetMathLibrary.MakeVector` (`KismetMathLibrary.RandomFloatInRange` _returnvalue _radius) (`KismetMathLibrary.RandomFloatInRange` _returnvalue _radius)) 0.0 (`self.Radius`)) (struct) (5.0 5.0 200.0)) false)))
    (:`then_1`
      (`self.DisplayCircle`))))