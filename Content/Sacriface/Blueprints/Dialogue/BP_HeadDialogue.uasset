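; BP_HeadDialogue drives the Head's staged dialogue, with later lines gated on kill progress in BPGMB_Default.
; Talk advances the index, then requires enough deer kills for the second line and ghost and centipede deaths for the third.
; A passing check triggers camera shake, a dialogue widget and a matching voiceline.
; After the third line, a long delay precedes setting MouthOpen on BP_TheHead's animation instance.
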(event `/Game/Sacriface/Blueprints/Dialogue/BPI_Dialogue.Talk`
  (bind _returnvalue (`self.K2_GetActorLocation`))
  (`/Engine/EditorBlueprintResources/StandardMacros.IncrementInt` (`self.DialogueIndex`)
    (:`  `
      (switch `int` (`self.DialogueIndex`)
        (:`0`
          (if (< (`self.DialogueIndex`) (`KismetArrayLibrary.Array_Length` (`self.Dialogue`))) :!label _label
            (`GameplayStatics.PlayWorldCameraShake` "/Game/Sacriface/Blueprints/Dialogue/BP_HeadCameraShake.BP_HeadCameraShake_C" (`PlayerCameraManager.GetCameraLocation` (`GameplayStatics.GetPlayerCameraManager` 0)) 0.0 50.0)
            (bind _returnvalue_2 (`|CreateWidget` "/Game/Sacriface/Blueprints/Dialogue/WBP_Dialogue.WBP_Dialogue_C" (`GameplayStatics.GetPlayerController` 0) (`|GetArrayItem` (`self.Dialogue`) (`self.DialogueIndex`))))
            (bind _output_get (set `self.DialogueUI` _returnvalue_2))
            (`UserWidget.AddToViewport` _output_get 0)
            (switch `int` (`self.DialogueIndex`)
              (:`0`
                (`GameplayStatics.PlaySoundAtLocation` "/Game/Sacriface/Audio/Voicelines/Head_Voicelines_1_SC.Head_Voicelines_1_SC" _returnvalue (struct) 1.0 1.0 0.0 null null null null))
              (:`1`
                (`GameplayStatics.PlaySoundAtLocation` "/Game/Sacriface/Audio/Voicelines/Head_Voicelines_2_SC.Head_Voicelines_2_SC" _returnvalue (struct) 1.0 1.0 0.0 null null null null))
              (:`2`
                (`GameplayStatics.PlaySoundAtLocation` "/Game/Sacriface/Audio/Voicelines/Head_Voicelines_3_SC.Head_Voicelines_3_SC" _returnvalue (struct) 1.0 1.0 0.0 null null null null)
                (`KismetSystemLibrary.Delay` 45.0)
                (bind _returnvalue_3 (`GameplayStatics.GetActorOfClass` "/Game/Sacriface/Characters/TheHead/BP_TheHead.BP_TheHead_C"))
                (bind _asabp_head (cast `/Game/Sacriface/Characters/TheHead/ABP_Head` (`SkeletalMeshComponent.GetAnimInstance` (`Character.Mesh` _returnvalue_3))))
                (set `/Game/Sacriface/Characters/TheHead/ABP_Head.MouthOpen` true _asabp_head)))))
        (:`1`
          (bind _asbpgmb_default (cast `/Game/Sacriface/Blueprints/BPGMB_Default` (`GameplayStatics.GetGameMode`)))
          (if (>= (`/Game/Sacriface/Blueprints/BPGMB_Default.DeerKilled` _asbpgmb_default) 5)
            (goto _label)))
        (:`2`
          (bind _asbpgmb_default_2 (cast `/Game/Sacriface/Blueprints/BPGMB_Default` (`GameplayStatics.GetGameMode`)))
          (if (and (`/Game/Sacriface/Blueprints/BPGMB_Default.GhostDead` _asbpgmb_default_2) (`/Game/Sacriface/Blueprints/BPGMB_Default.CentipedeDead` _asbpgmb_default_2))
            (goto _label)))))))

(fn `UserConstructionScript`)