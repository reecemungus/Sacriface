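; BP_Newspaper is a readable newspaper actor that sets up a ghost scare.
; Its ReadPaper event shows the WBP_Paper widget, plays a paper sound and destroys the Sphere component.
; After a fixed delay it removes the widget, then spawns BP_Ghost at GhostLocation with a creepy laugh.
; Nothing in this graph calls ReadPaper, and BeginPlay, overlap and Tick are empty.
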(event `/Game/Sacriface/Blueprints/BPI_Newspaper.Read Paper`
  (bind _ghostlocation (`self.GhostLocation`))
  (bind _returnvalue (`|CreateWidget` "/Game/Sacriface/UIAssets/WBP_Paper.WBP_Paper_C" (`GameplayStatics.GetPlayerController` 0)))
  (`UserWidget.AddToViewport` _returnvalue 0)
  (`ActorComponent.K2_DestroyComponent` (`self.Sphere`))
  (`GameplayStatics.PlaySoundAtLocation` "/Game/Sacriface/Audio/Cabin/Newspaper_SC.Newspaper_SC" (`self.K2_GetActorLocation`) (struct) 1.0 1.0 0.0 null null null null)
  (`KismetSystemLibrary.Delay` 10.0)
  (`Widget.RemoveFromParent` _returnvalue)
  (`|SpawnActorFromClass` "/Game/Sacriface/Characters/Ghost/BP_Ghost.BP_Ghost_C" (`KismetMathLibrary.MakeTransform` _ghostlocation) "AdjustIfPossibleButAlwaysSpawn" "MultiplyWithRoot" null null)
  (`GameplayStatics.PlaySoundAtLocation` "/Game/Sacriface/Audio/Ambience/Creepy_Laugh_SC.Creepy_Laugh_SC" _ghostlocation (struct) 1.0 1.0 0.0 null null null null))

(fn `UserConstructionScript`)