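; BP_Tree is a procedural tree actor, built entirely in the construction script with no active runtime logic.
; It spaces BranchAmount intervals along a spline, adding a random one of four instanced branch meshes at each point with random yaw and slight tilt.
; Scale grows with spline distance times SizeVector, rounded up to whole numbers.
; A Balls instance accompanies each branch at 1.5 times that scale; unseeded randomness reshuffles the layout on every reconstruction.
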(fn `UserConstructionScript`
  (bind _branchamount (`self.BranchAmount`))
  (bind _returnvalue (`KismetMathLibrary.MakeRotator` (`KismetMathLibrary.RandomFloatInRange` -15.0 15.0) (`KismetMathLibrary.RandomFloatInRange` -15.0 15.0) (`KismetMathLibrary.RandomFloatInRange` 0.0 360.0)))
  (`StaticMeshComponent.SetStaticMesh` (`self.Branch1`) "/Game/Sacriface/Meshes/Branches/Branches_Branch.Branches_Branch")
  (`StaticMeshComponent.SetStaticMesh` (`self.Branch2`) "/Game/Sacriface/Meshes/Branches/Branches_Branch_001.Branches_Branch_001")
  (`StaticMeshComponent.SetStaticMesh` (`self.Branch3`) "/Game/Sacriface/Meshes/Branches/Branches_Branch_002.Branches_Branch_002")
  (`StaticMeshComponent.SetStaticMesh` (`self.Branch4`) "/Game/Sacriface/Meshes/Branches/Branches_Branch_003.Branches_Branch_003")
  (for _index (range (+ _branchamount 1))
    (bind _returnvalue_2 (* _index (/ (`SplineComponent.GetSplineLength` (`self.Spline`)) _branchamount)))
    (bind _returnvalue_3 (`SplineComponent.GetLocationAtDistanceAlongSpline` (`self.Spline`) _returnvalue_2 "Local"))
    (bind _returnvalue_4 (`KismetMathLibrary.MakeVector` (`KismetMathLibrary.Conv_IntToDouble` (`KismetMathLibrary.FCeil` (.x (* (/ _returnvalue_2 1000.0) (`self.SizeVector`))))) (`KismetMathLibrary.Conv_IntToDouble` (`KismetMathLibrary.FCeil` (.y (* (/ _returnvalue_2 1000.0) (`self.SizeVector`))))) (`KismetMathLibrary.Conv_IntToDouble` (`KismetMathLibrary.FCeil` (.z (* (/ _returnvalue_2 1000.0) (`self.SizeVector`)))))))
    (`InstancedStaticMeshComponent.AddInstance` (`KismetArrayLibrary.Array_Random` (`|MakeArray` (`self.Branch1`) (`self.Branch2`) (`self.Branch3`) (`self.Branch4`))) (`KismetMathLibrary.MakeTransform` _returnvalue_3 _returnvalue _returnvalue_4) false)
    (`InstancedStaticMeshComponent.AddInstance` (`self.Balls`) (`KismetMathLibrary.MakeTransform` _returnvalue_3 _returnvalue (* _returnvalue_4 1.5)) false)))