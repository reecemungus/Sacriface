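; BP_SplineCyls is a construction-script tool that lines copies of a chosen mesh along a spline as instanced static meshes.
; Spacing comes from the mesh's unscaled X bounds plus an offset, setting how many instances fit the spline length.
; Each instance sits at its distance along the spline, aims at the next point, and gets a random roll within RollOffset plus a shared scale.
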(fn `GetLocationAtIndex`
  (params (Index :type Integer))
  (returns (ReturnValue :type "Vector Structure"))
  (return (`SplineComponent.GetLocationAtDistanceAlongSpline` (`self.Spline`) (* Index (`self.Spacing`)) "Local")))

(fn `UserConstructionScript`
  (locals (Insts :type Integer :default 0))
  (bind (_rolloffset_x _rolloffset_y) (`KismetMathLibrary.BreakVector` (`self.RollOffset`)))
  (bind (_min _max) (break `Box` (`StaticMesh.GetBoundingBox` (`self.Mesh`))))
  (`StaticMeshComponent.SetStaticMesh` (`self.InstancedStaticMesh`) (`self.Mesh`))
  (bind _output_get (set `self.Spacing` (+ (.x (- _max _min)) (`self.Offset`))))
  (bind _returnvalue (`KismetMathLibrary.FFloor` (/ (`SplineComponent.GetSplineLength` (`self.Spline`)) _output_get)))
  (set `local.Insts` _returnvalue)
  (for _index (range (+ _returnvalue 1))
    (bind _returnvalue_2 (`self.GetLocationAtIndex` _index))
    (bind (_returnvalue_roll _returnvalue_pitch _returnvalue_yaw) (`KismetMathLibrary.BreakRotator` (`KismetMathLibrary.MakeRotFromX` (- (`self.GetLocationAtIndex` (+ _index 1)) _returnvalue_2))))
    (`InstancedStaticMeshComponent.AddInstance` (`self.InstancedStaticMesh`) (`KismetMathLibrary.MakeTransform` _returnvalue_2 (`KismetMathLibrary.MakeRotator` (+ _returnvalue_roll (`KismetMathLibrary.RandomFloatInRange` _rolloffset_x _rolloffset_y)) (+ _returnvalue_pitch 0.0) (+ _returnvalue_yaw 0.0)) (`self.Scale`)) false)))