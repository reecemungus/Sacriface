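; AI controller for the Centipede that runs BT_Centipede on possess and reacts to perception of actors tagged Player.
; Successfully sensing the player clears EnemyTimer, while a failed stimulus starts it with the LineOfSightTimer delay.
; When the timer fires, it sets HasLineOfSight to true and writes the actor to EnemyActor on the Blackboard.
; No path here sets the Blackboard on a successful sense or resets HasLineOfSight to false.
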(event `self.ReceivePossess`
  (params (PossessedPawn :type "Pawn Object Reference"))
  (`self.RunBehaviorTree` "/Game/Sacriface/Characters/Centipede/AI/BT_Centipede.BT_Centipede"))

(event `self.AIPerception.OnTargetPerceptionUpdated`
  (params (Actor :type "Actor Object Reference") (Stimulus :type "AIStimulus Structure"))
  (bind _returnvalue (`self.ActorHasTag` Actor "Player"))
  (if _returnvalue
    (if (and _returnvalue (`.bSuccessfullySensed` (break `AIStimulus` Stimulus)))
      (`KismetSystemLibrary.K2_ClearAndInvalidateTimerHandle` (`self.EnemyTimer`))
      (else
        (bind _returnvalue_2 (`KismetSystemLibrary.K2_SetTimerDelegate` (delegate `StartEnemyTimer`) (`self.LineOfSightTimer`)))
        (set `self.EnemyTimer` _returnvalue_2)))))

(event `StartEnemyTimer`
  (bind _blackboard (`self.Blackboard`))
  (`BlackboardComponent.SetValueAsBool` _blackboard (`self.HasLineOfSight`) true)
  (`BlackboardComponent.SetValueAsObject` _blackboard (`self.EnemyActor`) (stale `self.AIPerception.OnTargetPerceptionUpdated` Actor)))

(fn `UserConstructionScript`)