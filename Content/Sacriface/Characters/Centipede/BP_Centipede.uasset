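; BP_Centipede is a centipede enemy character that plays a randomly pitched crawling sound every three seconds.
; It only loses health from damage types whose name contains "Shotgun", using a substring check.
; On death it disables capsule collision, messages its anim instance, spawns Niagara death effects at each mesh child component, hisses, notifies BPGMB_Default and destroys itself.
; An UpdateWalkSpeed event sets its movement speed.
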(event `self.ReceiveBeginPlay`
  (`KismetSystemLibrary.K2_SetTimerDelegate` (delegate `PlaySound`) 3.0 true))

(event `PlaySound`
  (`GameplayStatics.PlaySoundAtLocation` "/Game/Sacriface/Audio/Centipede/Centipede_Crawling_SC.Centipede_Crawling_SC" (`self.K2_GetActorLocation`) (struct) 1.0 (`KismetMathLibrary.RandomFloatInRange` 0.8 1.2) 0.0 null null null null))

(event `self.ReceiveAnyDamage`
  (params (Damage :type "Float (single-precision)") (DamageType :type "DamageType Object Reference") (InstigatedBy :type "Controller Object Reference") (DamageCauser :type "Actor Object Reference"))
  (if (`KismetStringLibrary.Contains` (`KismetSystemLibrary.GetObjectName` DamageType) "Shotgun")
    (bind _output_get (set `self.Health` (- (`self.Health`) Damage)))
    (if (<= _output_get 0.0)
      (`self.OnDeath`))))

(event `OnDeath`
  (`PrimitiveComponent.SetCollisionEnabled` (`self.CapsuleComponent`) "NoCollision")
  (message `/Game/Sacriface/Characters/BPI_ABPCanDie.On ABP Death` (`SkeletalMeshComponent.GetAnimInstance` (`self.Mesh`)))
  (for _array_element (`SceneComponent.GetChildrenComponents` (`self.Mesh`) false)
    (bind _returnvalue (`SceneComponent.K2_GetComponentLocation` _array_element))
    (`NiagaraFunctionLibrary.SpawnSystemAtLocation` "/Game/Sacriface/Particles/NS_CentipedeDeath.NS_CentipedeDeath" _returnvalue))
  (`GameplayStatics.PlaySoundAtLocation` "/Game/Sacriface/Audio/Centipede/Centipede_Hissing_2_SC.Centipede_Hissing_2_SC" _returnvalue (struct) 1.0 1.0 0.0 null null null null)
  (bind _asbpgmb_default (cast `/Game/Sacriface/Blueprints/BPGMB_Default` (`GameplayStatics.GetGameMode`)))
  (`/Game/Sacriface/Blueprints/BPGMB_Default.OnCentipedeDeath` _asbpgmb_default)
  (`self.K2_DestroyActor`))

(event `/Game/Sacriface/Characters/BPI_UpdateWalkSpeed.Update Walk Speed`
  (params (NewWalkSpeed :type "Float (double-precision)"))
  (set `CharacterMovementComponent.MaxWalkSpeed` NewWalkSpeed (`self.CharacterMovement`)))

(fn `UserConstructionScript`)